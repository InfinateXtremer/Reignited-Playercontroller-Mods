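; Tron suit lighting actor that recolors Spyro's body glow to match his companion Sparx and reacts to power-ups.
; Each Tick it finds Sparx among the player's child actors and flags a power-up when the body material is fireball, ice, poison or rage flames.
; Power-ups light the eyes and circuitry; otherwise Sparx's diffuse texture selects orange, blue or green glow, using dynamic materials created on demand.
; A SparxLightState save loader is defined but never called here.
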(event `ChangeSpyroColor`
  (params (NewColor :type "LinearColor Structure"))
  (bind _mesh (`Character.Mesh` (`GameplayStatics.GetPlayerCharacter` 0)))
  (bind _asmaterial_instance_dynamic (cast `MaterialInstanceDynamic` (`PrimitiveComponent.GetMaterial` _mesh 0))
    (:`then`
      (`MaterialInstanceDynamic.SetVectorParameterValue` _asmaterial_instance_dynamic "GlowColor" NewColor))
    (:`CastFailed`
      (bind _returnvalue (`KismetMaterialLibrary.CreateDynamicMaterialInstance` "/CPS1999_Spyro/Materials/MI_CPS1999_Spyro_Body.MI_CPS1999_Spyro_Body"))
      (`PrimitiveComponent.SetMaterial` _mesh 0 _returnvalue)
      (`MaterialInstanceDynamic.SetVectorParameterValue` _returnvalue "GlowColor" NewColor))))

(event `GetSpyroSparx`
  (bind _asbp_cps1999_playable (cast `/CPS1999_Spyro/Blueprints/BP_CPS1999_Playable` (`GameplayStatics.GetPlayerCharacter` 0) :!label _label)
    (:`then`
      (for _array_element (`self.GetAllChildActors` _asbp_cps1999_playable true)
        (bind _asbp_cps1194_sparx (cast `/CPS1194_SparxNew/Blueprints/BP_CPS1194_Sparx` _array_element :!label _label_2)
          (:`then`
            (set `self.Sparx` _asbp_cps1194_sparx)
            (set `self.GotSpyroAndSparx?` true))
          (:`CastFailed`
            (`KismetSystemLibrary.Delay` 1.0)
            (goto _label_2)))))
    (:`CastFailed`
      (`KismetSystemLibrary.Delay` 1.0)
      (goto _label))))

(event `self.ReceiveTick`
  (params (DeltaSeconds :type "Float (single-precision)"))
  (`self.GetSpyroSparx`)
  (`self.SetLeftEyeRedness`)
  (`self.SetRightEyeRedness`)
  (`self.GetPowerUp`)
  (`self.SetDiscTech`)
  (if (not (`self.Powerup?`))
    (bind _asmaterial_instance_dynamic (cast `MaterialInstanceDynamic` (`PrimitiveComponent.GetMaterial` (`self.GetComponentByClass` (`self.Sparx`) "/Script/Engine.SkeletalMeshComponent") 1)))
    (bind _returnvalue (`MaterialInstanceDynamic.K2_GetTextureParameterValue` _asmaterial_instance_dynamic "Diffuse Map"))
    (if (== _returnvalue "/CPS1194_SparxNew/Textures/T_CPS1194_SparxNew_C.T_CPS1194_SparxNew_C")
      (`self.ChangeSpyroColor` (struct :`R` 1.0 :`G` 0.674288 :`A` 1.0))
      (elif (== _returnvalue "/CPS1194_SparxNew/Textures/T_CPS1194_SparxNew_C_Blue.T_CPS1194_SparxNew_C_Blue")
        (`self.ChangeSpyroColor` (struct :`G` 0.188477 :`B` 1.0 :`A` 1.0))
        (else
          (`self.ChangeSpyroColor` (struct :`R` 0.251143 :`G` 1.0 :`A` 1.0)))))))

(event `GetPowerUp`
  (bind _returnvalue (`PrimitiveComponent.GetMaterial` (`Character.Mesh` (`GameplayStatics.GetPlayerCharacter` 0)) 0))
  (if (or (== _returnvalue "/CPS1999_Spyro/Materials/MI_CPS1999_Spyro_Fireball.MI_CPS1999_Spyro_Fireball") (== _returnvalue "/CPS1999_Spyro/Materials/MI_CPS1999_Spyro_Ice.MI_CPS1999_Spyro_Ice") (== _returnvalue "/CPS1999_Spyro/Materials/MI_CPS1999_Spyro_Poison.MI_CPS1999_Spyro_Poison") (== _returnvalue "/CPS1999_Spyro/Materials/MI_CPS1999_Spyro_RageFlames.MI_CPS1999_Spyro_RageFlames"))
    (set `self.Powerup?` true)
    (else
      (set `self.Powerup?` false))))

(event `SetDiscTech`
  (bind _mesh (`Character.Mesh` (`GameplayStatics.GetPlayerCharacter` 0)))
  (bind _asmaterial_instance_dynamic (cast `MaterialInstanceDynamic` (`PrimitiveComponent.GetMaterial` _mesh 4))
    (:`then`
      (if (`self.Powerup?`)
        (`MaterialInstanceDynamic.SetScalarParameterValue` _asmaterial_instance_dynamic "Opacity" 1.0)
        (else
          (`MaterialInstanceDynamic.SetScalarParameterValue` _asmaterial_instance_dynamic "Opacity" 0.0))))
    (:`CastFailed`
      (bind _returnvalue (`KismetMaterialLibrary.CreateDynamicMaterialInstance` "/Game/Tron/Disc/M_Circuitry.M_Circuitry"))
      (`PrimitiveComponent.SetMaterial` _mesh 4 _returnvalue)
      (if (`self.Powerup?`)
        (`MaterialInstanceDynamic.SetScalarParameterValue` _returnvalue "Opacity" 1.0)
        (else
          (`MaterialInstanceDynamic.SetScalarParameterValue` _returnvalue "Opacity" 0.0))))))

(event `SetLeftEyeRedness`
  (bind _mesh (`Character.Mesh` (`GameplayStatics.GetPlayerCharacter` 0)))
  (bind _asmaterial_instance_dynamic (cast `MaterialInstanceDynamic` (`PrimitiveComponent.GetMaterial` _mesh 1))
    (:`then`
      (if (`self.Powerup?`)
        (`MaterialInstanceDynamic.SetScalarParameterValue` _asmaterial_instance_dynamic "EmissiveStrenght" 20.0)
        (else
          (`MaterialInstanceDynamic.SetScalarParameterValue` _asmaterial_instance_dynamic "EmissiveStrenght" 0.0))))
    (:`CastFailed`
      (bind _returnvalue (`KismetMaterialLibrary.CreateDynamicMaterialInstance` "/CPS1999_Spyro/Materials/MI_CPS1999_Spyro_Eye_L.MI_CPS1999_Spyro_Eye_L"))
      (`PrimitiveComponent.SetMaterial` _mesh 1 _returnvalue)
      (if (`self.Powerup?`)
        (`MaterialInstanceDynamic.SetScalarParameterValue` _returnvalue "EmissiveStrenght" 20.0)
        (else
          (`MaterialInstanceDynamic.SetScalarParameterValue` _returnvalue "EmissiveStrenght" 0.0))))))

(event `SetRightEyeRedness`
  (bind _mesh (`Character.Mesh` (`GameplayStatics.GetPlayerCharacter` 0)))
  (bind _asmaterial_instance_dynamic (cast `MaterialInstanceDynamic` (`PrimitiveComponent.GetMaterial` _mesh 2))
    (:`then`
      (if (`self.Powerup?`)
        (`MaterialInstanceDynamic.SetScalarParameterValue` _asmaterial_instance_dynamic "EmissiveStrenght" 20.0)
        (else
          (`MaterialInstanceDynamic.SetScalarParameterValue` _asmaterial_instance_dynamic "EmissiveStrenght" 0.0))))
    (:`CastFailed`
      (bind _returnvalue (`KismetMaterialLibrary.CreateDynamicMaterialInstance` "/CPS1999_Spyro/Materials/MI_CPS1999_Spyro_Eye_R.MI_CPS1999_Spyro_Eye_R"))
      (`PrimitiveComponent.SetMaterial` _mesh 2 _returnvalue)
      (if (`self.Powerup?`)
        (`MaterialInstanceDynamic.SetScalarParameterValue` _returnvalue "EmissiveStrenght" 20.0)
        (else
          (`MaterialInstanceDynamic.SetScalarParameterValue` _returnvalue "EmissiveStrenght" 0.0))))))

(fn `GetSaveGame`
  (bind _returnvalue (`GameplayStatics.LoadGameFromSlot` "SparxLightState"))
  (bind _assparx_light_save (cast `/Game/SparxColor/SparxLight_Save` _returnvalue)
    (:`then`
      (set `self.SaveInstance` _assparx_light_save))
    (:`CastFailed`
      (bind _returnvalue_2 (`GameplayStatics.CreateSaveGameObject` "/Game/SparxColor/SparxLight_Save.SparxLight_Save_C"))
      (bind _assparx_light_save_2 (cast `/Game/SparxColor/SparxLight_Save` _returnvalue_2))
      (set `self.SaveInstance` _assparx_light_save_2)))
  (return))

(fn `UserConstructionScript`)