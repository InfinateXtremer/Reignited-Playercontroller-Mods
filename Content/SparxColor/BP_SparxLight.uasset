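; BP_SparxLight adds a colored point light to Spyro's Sparx companion, found among the player pawn's child actors.
; Tick and a looping timer keep the light created and attached to Sparx's mesh, whose shadow casting is disabled.
; In default mode, color and intensity follow Sparx's current diffuse texture.
; U opens a LightColor widget, notify events apply color and brightness changes, H toggles the light, and settings load from a save slot.
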(event `GetSpyroSparx`
  (bind _asbp_cps1999_playable (cast `/CPS1999_Spyro/Blueprints/BP_CPS1999_Playable` (`GameplayStatics.GetPlayerCharacter` 0) :!label _label)
    (:`then`
      (for _array_element (`self.GetAllChildActors` _asbp_cps1999_playable true)
        (bind _asbp_cps1194_sparx (cast `/CPS1194_SparxNew/Blueprints/BP_CPS1194_Sparx` _array_element :!label _label_2)
          (:`then`
            (set `self.Sparx` _asbp_cps1194_sparx)
            (set `self.GotSpyroAndSparx?` true))
          (:`CastFailed`
            (`KismetSystemLibrary.Delay` 1.0)
            (goto _label_2)))))
    (:`CastFailed`
      (`KismetSystemLibrary.Delay` 1.0)
      (goto _label))))

(event `Reattach`
  ;[1 1 1] Not used
  (`SceneComponent.K2_SetWorldLocation` (`self.SparxLight`) (`self.K2_GetActorLocation` (`self.Sparx`)) false false)
  (`SceneComponent.K2_AttachToComponent` (`self.SparxLight`) (`self.GetComponentByClass` (`self.Sparx`) "/Script/Engine.SkeletalMeshComponent") "None" "SnapToTarget" "SnapToTarget" "SnapToTarget" true))

(event `/Game/SparxColor/ISparxLight.INotifyLightColorChanged`
  (params (NewSparxColor :type "Color Structure"))
  (`self.GetSaveGame`)
  (if (`/Game/SparxColor/SparxLight_Save.CustomColor?` (`self.SaveInstance`))
    (set `self.DefaultColor?` false)
    (else
      (set `self.DefaultColor?` true)))
  (`LightComponent.SetLightColor` (`self.SparxLight`) (`KismetMathLibrary.Conv_ColorToLinearColor` NewSparxColor) true))

(event `self.ReceiveBeginPlay`
  (bind _saveinstance (`self.SaveInstance`))
  (`self.GetSaveGame` :!label _label_3)
  (if (`self.GotSpyroAndSparx?`) :!label _label_4
    (`self.CreateSparxLight`)
    (`KismetSystemLibrary.K2_SetTimer` null "CreateSparxLight" 1.0 true)
    (if (`/Game/SparxColor/SparxLight_Save.CustomColor?` _saveinstance)
      (`LightComponent.SetLightColor` (`self.SparxLight`) (`KismetMathLibrary.Conv_ColorToLinearColor` (`/Game/SparxColor/SparxLight_Save.LightColor` _saveinstance)) true)
      (else
        (set `self.DefaultColor?` true)
        (`LightComponent.SetIntensity` (`self.SparxLight`) (`/Game/SparxColor/SparxLight_Save.LightIntensity` (`self.SaveInstance`)))))
    (else
      (`KismetSystemLibrary.Delay` 1.0)
      (goto _label_4))))

(event `self.K2_OnReset`
  (goto _label_3))

(event `self.ReceiveEndPlay`
  (params (EndPlayReason :type "EEndPlayReason Enum" :default "Destroyed"))
  (goto _label_3))

(event `CreateSparxLight`
  (bind _returnvalue (`self.GetComponentByClass` (`self.Sparx`) "/Script/Engine.SkeletalMeshComponent"))
  (`/Engine/EditorBlueprintResources/StandardMacros.IsValid` (`self.SparxLight`)
    (:`Is Valid`
      (`SceneComponent.K2_AttachToComponent` (`self.SparxLight`) (`self.GetComponentByClass` (`self.Sparx`) "/Script/Engine.SkeletalMeshComponent") "None" "SnapToTarget" "SnapToTarget" "SnapToTarget" true))
    (:`Is Not Valid`
      (bind _returnvalue_2 (`AddComponent|NODE_AddPointLightComponent-7` :`self` (`self.Sparx`) :`bManualAttachment` true))
      (set `self.SparxLight` _returnvalue_2)
      (`PrimitiveComponent.SetCastShadow` _returnvalue false)
      (`SceneComponent.K2_AttachToComponent` (`self.SparxLight`) _returnvalue "None" "SnapToTarget" "SnapToTarget" "SnapToTarget" true)
      (`LightComponent.SetIntensity` (`self.SparxLight`) (`/Game/SparxColor/SparxLight_Save.LightIntensity` (`self.SaveInstance`))))))

(event `Key|U` :consume false :overrideparent false
  (params (Key :type "Key Structure"))
  (bind _returnvalue (`GameplayStatics.GetPlayerController` 0))
  (:`Pressed`
    (bind _returnvalue_2 (`|CreateWidget` "/Game/SparxColor/LightColor.LightColor_C"))
    (bind _output_get (set `self.ColorWidget` _returnvalue_2))
    (`UserWidget.AddToViewport` _output_get 0)
    (set `PlayerController.bShowMouseCursor` true _returnvalue)
    (`WidgetBlueprintLibrary.SetInputMode_UIOnlyEx` _returnvalue _output_get)))

(event `Key|H` :consume false :overrideparent false
  (params (Key :type "Key Structure"))
  (bind _sparxlight (`self.SparxLight`))
  (bind _saveinstance (`self.SaveInstance`))
  ;[1 1 1] Turning Light On And Off, No need to use this anymore
  (:`Pressed`
    (`/Engine/EditorBlueprintResources/StandardMacros.IsValid` (`self.Sparx`)
      (:`Is Valid`
        (if (== (`LightComponentBase.Intensity` (`self.SparxLight`)) (`self.DefaultIntensity`))
          (`LightComponent.SetIntensity` _sparxlight 0.0)
          (set `/Game/SparxColor/SparxLight_Save.LightOn?` false _saveinstance)
          (`GameplayStatics.SaveGameToSlot` _saveinstance "SparxLightState")
          (else
            (`LightComponent.SetIntensity` _sparxlight (`self.DefaultIntensity`))
            (set `/Game/SparxColor/SparxLight_Save.LightOn?` true _saveinstance)
            (`GameplayStatics.SaveGameToSlot` _saveinstance "SparxLightState")))))))

(event `self.ReceiveTick`
  (params (DeltaSeconds :type "Float (single-precision)"))
  (bind _sparxlight (`self.SparxLight`))
  (bind _sparxlight_2 (`self.SparxLight`))
  (bind _sparxlight_3 (`self.SparxLight`))
  (`self.CreateSparxLight`)
  (`self.GetSpyroSparx`)
  (if (`self.DefaultColor?`)
    (bind _asmaterial_instance_dynamic (cast `MaterialInstanceDynamic` (`PrimitiveComponent.GetMaterial` (`self.GetComponentByClass` (`self.Sparx`) "/Script/Engine.SkeletalMeshComponent") 1)))
    (bind _returnvalue (`MaterialInstanceDynamic.K2_GetTextureParameterValue` _asmaterial_instance_dynamic "Diffuse Map"))
    (if (== _returnvalue "/CPS1194_SparxNew/Textures/T_CPS1194_SparxNew_C.T_CPS1194_SparxNew_C")
      (`LightComponent.SetLightColor` _sparxlight_2 (struct :`R` 1.0 :`G` 0.396765 :`A` 1.0) true)
      (`LightComponent.SetIntensity` _sparxlight_2 1.0)
      (elif (== _returnvalue "/CPS1194_SparxNew/Textures/T_CPS1194_SparxNew_C_Blue.T_CPS1194_SparxNew_C_Blue")
        (`LightComponent.SetLightColor` _sparxlight_3 (struct :`G` 0.167027 :`B` 1.0 :`A` 1.0) true)
        (`LightComponent.SetIntensity` _sparxlight_3 0.7)
        (else
          (`LightComponent.SetLightColor` _sparxlight (struct :`R` 0.209955 :`G` 1.0 :`A` 1.0) true)
          (`LightComponent.SetIntensity` _sparxlight 0.5))))))

(event `/Game/SparxColor/ISparxLight.INotifyBrightness`
  (params (BrightnessValue :type "Float (single-precision)"))
  (`LightComponent.SetIntensity` (`self.SparxLight`) (`KismetMathLibrary.NormalizeToRange` BrightnessValue 0.0 1.0)))

(fn `GetSaveGame`
  (bind _returnvalue (`GameplayStatics.LoadGameFromSlot` "SparxLightState"))
  (bind _assparx_light_save (cast `/Game/SparxColor/SparxLight_Save` _returnvalue)
    (:`then`
      (set `self.SaveInstance` _assparx_light_save))
    (:`CastFailed`
      (bind _returnvalue_2 (`GameplayStatics.CreateSaveGameObject` "/Game/SparxColor/SparxLight_Save.SparxLight_Save_C"))
      (bind _assparx_light_save_2 (cast `/Game/SparxColor/SparxLight_Save` _returnvalue_2))
      (set `self.SaveInstance` _assparx_light_save_2)))
  (return))

(fn `UserConstructionScript`)